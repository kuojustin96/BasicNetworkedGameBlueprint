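; Grapple gun weapon that launches the owning player toward the point struck by its hitscan shot.
; A blocking hit places the cable end and hook mesh, then applies a velocity-change impulse along the hit direction, biased sideways by strafe input.
; ShowGrappleHook toggles both visuals and the owner's movement mode, switching to Flying on a hit and Falling when the server receives fire end.
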(event `self.ReceiveBeginPlay`
  ;[1 1 1] Set default visibility value
  (`SceneComponent.SetVisibility` (`self.GrappleCable`) false false)
  (`SceneComponent.SetVisibility` (`self.GrappleEndMesh`) false false))

(event `self.Local_OnFireStart`
  ;[1 1 1] Run functions when the weapon is fired/stops firing
  (`self.ShootHitscan` true))

(event `self.Server_OnFireEnd`
  ;[1 1 1] Run functions when the weapon is fired/stops firing
  (`parent.Server_OnFireEnd`)
  (`self.ShowGrappleHook` false))

(event `self.OnHitscanHit`
  (params (HitResult :type "HitResult Structure"))
  (bind _returnvalue (`self.GetOwner`))
  ;[1 1 1] Set the grapple end point, ideally would like to have a spline mesh to show the "grapple"
  (if HitResult_bBlockingHit
    (set `CableComponent.EndLocation` (`KismetMathLibrary.InverseTransformLocation` (`self.GetTransform`) HitResult_ImpactPoint) (`self.GrappleCable`))
    (`SceneComponent.K2_SetWorldLocation` (`self.GrappleEndMesh`) HitResult_ImpactPoint false false)
    (bind _asbp_vtplayer_character (cast `/Game/GameFiles/Blueprints/BP_VTPlayerCharacter` _returnvalue))
    (`CharacterMovementComponent.AddImpulse` (`Character.CharacterMovement` _asbp_vtplayer_character) (* (`KismetMathLibrary.Normal` (+ (`KismetMathLibrary.GetDirectionUnitVector` (`self.K2_GetActorLocation` _returnvalue) HitResult_ImpactPoint) (* (* (`self.GetActorRightVector` _returnvalue) (`self.GetInputAxisValue`)) 0.7))) (`self.GrappleForce`)) true)
    (`self.ShowGrappleHook` true)))

(fn `ShowGrappleHook`
  (params (bIsVisible :type Boolean))
  (bind _returnvalue (`self.GetOwner`))
  (bind _grapplecable (`self.GrappleCable`))
  (bind _grappleendmesh (`self.GrappleEndMesh`))
  ;[1 1 1] Used to control grapple hook visibility
  (if bIsVisible
    (`SceneComponent.SetVisibility` _grapplecable true false)
    (`SceneComponent.SetVisibility` _grappleendmesh true false)
    (bind _asbp_vtplayer_character (cast `/Game/GameFiles/Blueprints/BP_VTPlayerCharacter` _returnvalue))
    (`CharacterMovementComponent.SetMovementMode` (`Character.CharacterMovement` _asbp_vtplayer_character) "MOVE_Flying" 0)
    (else
      (`SceneComponent.SetVisibility` _grapplecable false false)
      (`SceneComponent.SetVisibility` _grappleendmesh false false)
      (bind _asbp_vtplayer_character_2 (cast `/Game/GameFiles/Blueprints/BP_VTPlayerCharacter` _returnvalue))
      (`CharacterMovementComponent.SetMovementMode` (`Character.CharacterMovement` _asbp_vtplayer_character_2) "MOVE_Falling" 0))))

(fn `UserConstructionScript`
  (`parent.UserConstructionScript`))
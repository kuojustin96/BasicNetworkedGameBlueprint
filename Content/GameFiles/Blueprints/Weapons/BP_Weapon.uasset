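; Base weapon Blueprint that handles held-trigger firing of projectiles and offers a hitscan trace for child classes.
; Server fire events forward to client events, which toggle a held flag driving a delayed while-loop macro that repeatedly spawns projectiles from the first-person mesh socket.
; ShootHitscan traces forward from the player camera and can trigger OnHitscanHit, an empty hook alongside Local_OnFireStart for children to extend.
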(event `Server_OnFireStart`
  (params (Projectile :type "/Game/GameFiles/Blueprints/Weapons/BP_Projectile Class Reference"))
  ;[1 1 1] Weapon OnFire functionality
  (`self.Client_OnFireStart` Projectile))

(event `Client_OnFireStart`
  (params (Projectile :type "/Game/GameFiles/Blueprints/Weapons/BP_Projectile Class Reference"))
  ;[1 1 1] Weapon OnFire functionality
  (`self.Local_OnFireStart`)
  (set `self.bIsFireHeldDown` true)
  (if (`KismetSystemLibrary.IsValidClass` Projectile)
    (`self.WhileLoopWithDelay` (`self.TimeBetweenShots`) (`self.bIsFireHeldDown`)
      (:`LoopBody`
        (`self.SpawnProjectile` Projectile)))))

(event `Server_OnFireEnd`
  ;[1 1 1] Weapon OnFire finished functionality
  (`self.Client_OnFireEnd`))

(event `Client_OnFireEnd`
  ;[1 1 1] Weapon OnFire finished functionality
  (set `self.bIsFireHeldDown` false))

(event `OnHitscanHit`
  (params (HitResult :type "HitResult Structure"))
  ;[1 1 1] Can be used by children, could also play generics here like VFX or SFX
)

(event `Local_OnFireStart`
  ;[1 1 1] Can be used by children, could also play generics here like VFX or SFX
)

(fn `ShootHitscan`
  (params (bCallEvent :type Boolean :default true))
  (returns (HitResult :type "HitResult Structure"))
  (bind _playercamera (`/Game/GameFiles/Blueprints/BP_VTPlayerCharacter.PlayerCamera` (`self.PlayerCharacter`)))
  (bind _returnvalue (`SceneComponent.K2_GetComponentLocation` _playercamera))
  ;[1 1 1] Shoots a raycast forward from the player camera
  (bind _outhit (`KismetSystemLibrary.LineTraceSingle` _returnvalue (+ _returnvalue (* (`KismetMathLibrary.GetForwardVector` (`SceneComponent.K2_GetComponentRotation` _playercamera)) (`self.HitscanRange`))) "TraceTypeQuery1" false (`|MakeArray` (`self.GetOwner`))))
  (if bCallEvent
    (`self.OnHitscanHit` _outhit))
  (return _outhit))

(fn `SpawnProjectile`
  (params (ProjectileClass :type "/Game/GameFiles/Blueprints/Weapons/BP_Projectile Class Reference"))
  (bind _returnvalue (`|SpawnActorFromClass` ProjectileClass (`KismetMathLibrary.MakeTransform` (`SceneComponent.GetSocketLocation` (`self.WeaponMesh1P`) (`self.WeaponSocketName`))) "AlwaysSpawn" "OverrideRootScale" null null))
  (`self.SetOwner` _returnvalue (`self.GetOwner`))
  (`/Game/GameFiles/Blueprints/Weapons/BP_Projectile.EnableProjectile` _returnvalue))

(fn `UserConstructionScript`)
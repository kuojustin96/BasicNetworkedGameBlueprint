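; Projectile actor for weapons that flies along the aim of the player who owns it.
; EnableProjectile casts the owner to BP_VTPlayerCharacter and sets the projectile movement velocity to that player camera's forward vector times ProjectileSpeed.
; The collision component's hit event destroys the actor, with no owner check or damage logic in the graph.
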(event `EnableProjectile`
  ;[1 1 1] Set projectile velocity based on the player's facing direction
  (set `MovementComponent.Velocity` (* (`KismetMathLibrary.GetForwardVector` (`SceneComponent.K2_GetComponentRotation` (`/Game/GameFiles/Blueprints/BP_VTPlayerCharacter.PlayerCamera` (cast `/Game/GameFiles/Blueprints/BP_VTPlayerCharacter` (`self.GetOwner`) :!pure true)))) (`self.ProjectileSpeed`)) (`self.ProjectileMovement`)))

(event `self.ProjectileCollision.OnComponentHit`
  (params (HitComponent :type "PrimitiveComponent Object Reference") (OtherActor :type "Actor Object Reference") (OtherComp :type "PrimitiveComponent Object Reference") (NormalImpulse :type "Vector Structure") (Hit :type "HitResult Structure (by ref)"))
  ;[1 1 1] Destory projectile if it hits something that isn't the player who shot it
  (`self.K2_DestroyActor`))

(fn `UserConstructionScript`)
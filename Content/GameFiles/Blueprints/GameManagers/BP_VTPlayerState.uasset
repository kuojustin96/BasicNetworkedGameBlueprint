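; BP_VTPlayerState is the player state that holds the player's score and exposes set, add and get functions for it.
; On BeginPlay it zeroes the score and caches player 0's BP_VTPlayerCharacter.
; Setting or adding points passes the new total to the character's UpdatePlayerScore.
; An OnRep handler for PlayerScore also writes the value straight to the character's GameplayUI.
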(event `self.ReceiveBeginPlay`
  ;[1 1 1] Ensure score is set to 0 when the game starts
  (set `self.PlayerScore` 0)
  ;[1 1 1] Get the player character and save to a variable for future use, set score to start the game
  (bind _asbp_vtplayer_character (cast `/Game/GameFiles/Blueprints/BP_VTPlayerCharacter` (`GameplayStatics.GetPlayerCharacter` 0)))
  (bind _output_get (set `self.PlayerCharacter` _asbp_vtplayer_character))
  (`/Game/GameFiles/Blueprints/BP_VTPlayerCharacter.UpdatePlayerScore` _output_get (`self.PlayerScore`)))

(fn `Add Player Score`
  (params (`Value To Add` :type Integer))
  (bind _output_get (set `self.PlayerScore` (+ `Value To Add` (`self.PlayerScore`))))
  (`/Game/GameFiles/Blueprints/BP_VTPlayerCharacter.UpdatePlayerScore` (`self.PlayerCharacter`) _output_get))

(fn `GetPlayerScore`
  (returns (Score :type Integer))
  (return (`self.PlayerScore`)))

(fn `OnRep_PlayerScore`
  (`/Game/GameFiles/Blueprints/UI/WBP_MainUI.Update Score` (`/Game/GameFiles/Blueprints/BP_VTPlayerCharacter.GameplayUI` (`self.PlayerCharacter`)) (`self.PlayerScore`)))

(fn `SetPlayerScore`
  (params (Score :type Integer))
  (bind _output_get (set `self.PlayerScore` Score))
  (`/Game/GameFiles/Blueprints/BP_VTPlayerCharacter.UpdatePlayerScore` (`self.PlayerCharacter`) _output_get))

(fn `UserConstructionScript`)
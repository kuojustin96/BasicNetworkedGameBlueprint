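; Game state that runs the match countdown and decides when the game is over.
; On BeginPlay it takes the time limit from BP_VTGameMode, so only the server runs the looping one-second timer.
; CurrentGameTime's RepNotify pushes the time to the player-0 character's UI.
; Game over triggers through that character at zero or once all players finish; earlier finishers lose input and see a finished screen.
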(event `self.ReceiveBeginPlay`
  ;[1 1 1] Game Timer Setup
  (bind _asbp_vtgame_mode (cast `/Game/GameFiles/Blueprints/GameManagers/BP_VTGameMode` (`GameplayStatics.GetGameMode`)))
  (bind _output_get (set `self.GameTimeLimit` (+ (`/Game/GameFiles/Blueprints/GameManagers/BP_VTGameMode.GameTimeLimit` _asbp_vtgame_mode) 1.0)))
  (set `self.CurrentGameTime` _output_get)
  (`self.StartGameTimer`))

(event `StartGameTimer`
  ;[1 1 1] Game Timer Countdown
  (bind _returnvalue (`KismetSystemLibrary.K2_SetTimerDelegate` (delegate `OnGameTimerEnd`) 1.0 true))
  (set `self.TimerHandle` _returnvalue)
  (cast `/Game/GameFiles/Blueprints/GameManagers/BP_VTPlayerState` (`|GetArrayItem` (`self.PlayerArray`) 1)))

(event `OnGameTimerEnd`
  ;[1 1 1] Game Timer Countdown
  (bind _output_get (set `self.CurrentGameTime` (- (`self.CurrentGameTime`) 1.0)))
  (if (<= _output_get 0.0)
    (`KismetSystemLibrary.K2_ClearAndInvalidateTimerHandle` (`self.TimerHandle`))
    (`self.ShowGameOverUI`)))

(fn `OnPlayerFinished`
  (params (PlayerCharacter :type "/Game/GameFiles/Blueprints/BP_VTPlayerCharacter Object Reference"))
  (bind _numplayersfinished (`self.NumPlayersFinished`))
  (`/Engine/EditorBlueprintResources/StandardMacros.IncrementInt` _numplayersfinished
    (:`  `
      (if (>= _numplayersfinished (`KismetArrayLibrary.Array_Length` (`self.PlayerArray`)))
        (`self.ShowGameOverUI`)
        (else
          (`self.DisableInput` PlayerCharacter (cast `/Game/GameFiles/Blueprints/GameManagers/BP_VTPlayerController` (`Pawn.GetController` PlayerCharacter) :!pure true))
          (`/Game/GameFiles/Blueprints/BP_VTPlayerCharacter.ShowPlayerFinishedUI` PlayerCharacter))))))

(fn `OnRep_CurrentGameTime`
  (bind _asbp_vtplayer_character (cast `/Game/GameFiles/Blueprints/BP_VTPlayerCharacter` (`GameplayStatics.GetPlayerCharacter` 0)))
  (`/Game/GameFiles/Blueprints/BP_VTPlayerCharacter.UpdateGameplayUITimer` _asbp_vtplayer_character (`self.CurrentGameTime`)))

(fn `ShowGameOverUI`
  (bind _asbp_vtplayer_character (cast `/Game/GameFiles/Blueprints/BP_VTPlayerCharacter` (`GameplayStatics.GetPlayerCharacter` 0)))
  (`/Game/GameFiles/Blueprints/BP_VTPlayerCharacter.Server_TriggerGameOverUI` _asbp_vtplayer_character 0))

(fn `UserConstructionScript`)
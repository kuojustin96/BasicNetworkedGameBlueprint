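; BP_Collectable is the base class for collectable power-up pickups that spin cosmetically in the world.
; On sphere overlap, only the locally controlled BP_VTPlayerCharacter reacts, sending the player and collectable names to the server through ServerOnCollectablePickedUp.
; It then calls ApplyPowerUp with the player state, an event children override for their effect while the base implementation destroys the actor.
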(event `self.ReceiveTick`
  (params (DeltaSeconds :type "Float (single-precision)"))
  ;[1 1 1] Basic cosmetic rotation
  (`SceneComponent.K2_AddRelativeRotation` (`self.DefaultSceneRoot`) (struct :`Yaw` 1.0) false false))

(event `self.SphereCollision.OnComponentBeginOverlap`
  (params (OverlappedComponent :type "PrimitiveComponent Object Reference") (OtherActor :type "Actor Object Reference") (OtherComp :type "PrimitiveComponent Object Reference") (OtherBodyIndex :type Integer) (bFromSweep :type Boolean) (SweepResult :type "HitResult Structure (by ref)"))
  ;[1 1 1] Apply power up when player collects the collectable
  (bind _asbp_vtplayer_character (cast `/Game/GameFiles/Blueprints/BP_VTPlayerCharacter` OtherActor))
  (if (`Pawn.IsLocallyControlled` _asbp_vtplayer_character)
    (bind _asbp_vtplayer_state (cast `/Game/GameFiles/Blueprints/GameManagers/BP_VTPlayerState` (`Pawn.PlayerState` _asbp_vtplayer_character)))
    (`/Game/GameFiles/Blueprints/BP_VTPlayerCharacter.Server_OnCollectablePickedUp` _asbp_vtplayer_character (`PlayerState.GetPlayerName` _asbp_vtplayer_state) (`self.CollectableName`) _asbp_vtplayer_character)
    (`self.ApplyPowerUp` _asbp_vtplayer_state)))

(event `ApplyPowerUp`
  (params (PlayerState :type "/Game/GameFiles/Blueprints/GameManagers/BP_VTPlayerState Object Reference"))
  ;[1 1 1] Functionality implemented in children, if using C++, could be replaced with a BlueprintNativeEvent so you don't have to call a parent call in the child
  (`self.K2_DestroyActor`))

(fn `UserConstructionScript`)